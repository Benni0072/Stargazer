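; BP_Cat is an interactable cat that meows and shows a floating heart when the player interacts with it.
; Interact calls PlayCatSound, which plays a mouth animation and sound, then returns to the looping idle after a short delay.
; A timeline drives a dynamic material's fade and moves the heart upward with sideways motion.
; A Pressed flag blocks retriggering until a delay chained from the timeline update resets it.
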(event Custom|PlayCatSound
  (bind _heartpartikle (Variables|Default|GetHeartPartikle))
  (if (Variables|Default|Getpressed)
    (Variables|Default|Setpressed false)
    (Components|Animation|PlayAnimation (Variables|Default|GetCat_002_Plane) "/Game/Assets/Cat/NewTry/Cat_002_Plane_Anim_Mouth.Cat_002_Plane_Anim_Mouth" false)
    (Audio|PlaySound2D "/Game/Sound/SFX/Cat/SC_CatMouw.SC_CatMouw" 1.0 1.0 0.0 0 0)
    (Utilities|FlowControl|Sequence
      (:then_0
        (bind _returnvalue (Rendering|Material|CreateDynamicMaterialInstance (Variables|Default|GetHeartPartikle) 0 "/Game/Materials/MM_Fade.MM_Fade" "None" :!class /Script/Engine.PrimitiveComponent))
        (bind (_direction _heart _heartmovement2 _heart_movement) (Timeline|Animation%20Heart PlayFromStart)
          (:Update
            (Rendering|Material|SetScalarParameterValue _returnvalue "Fade" _heart :!class /Script/Engine.MaterialInstanceDynamic)
            (Transformation|SetRelativeLocation _heartpartikle (Math|Vector|MakeVector (* _heartmovement2 (Variables|Default|Getlenght)) (.y (Variables|/Script/Engine.SceneComponent|GetRelativeLocation _heartpartikle)) (Math|Float|Lerp (Variables|Default|GetStartPosition) (+ (Variables|Default|GetStartPosition) 5e+01) _heart_movement)) false false)
            (Utilities|FlowControl|Delay 2.0)
            (Variables|Default|Setpressed true))))
      (:then_1
        (Utilities|FlowControl|Delay 0.7)
        (Components|Animation|PlayAnimation (Variables|Default|GetCat_002_Plane) "/Game/Assets/Cat/NewTry/Cat_002_Plane_Anim_Idle002.Cat_002_Plane_Anim_Idle002" true)))))

(event EventBeginPlay
  (Variables|Default|SetStartPosition (.z (Variables|/Script/Engine.SceneComponent|GetRelativeLocation (Variables|Default|GetHeartPartikle)))))

(fn ConstructionScript)

(fn Interact
  (params (PlayerCharacter :type BP%20First%20Person%20Character%20Object%20Reference))
  (CallFunction|PlayCatSound)
  (return false))
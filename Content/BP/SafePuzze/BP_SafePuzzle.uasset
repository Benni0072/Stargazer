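; Possessable safe puzzle where the player rotates a wheel and confirms to check its face against the correct code.
; Extends a parent puzzle's interact and return logic with wheel highlighting, a controls widget and Enhanced Input context swaps.
; A correct code blends to a camera, swings the door open via timeline, returns control and disables re-possession.
; Wrong codes, and interactions once opened, show data-table textboxes.
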(event Custom|EndText
  (Widget|RemovefromParent (Variables|Default|GetTextbox))
  (Input|AddMappingContext (PlayerController|LocalPlayerSubsystems|GetEnhancedInputLocalPlayerSubsystem (Game|GetPlayerController 0)) (Variables|Default|GetPuzzleMapping%20Context) 0 "(bIgnoreAllPressedKeysUntilRelease=True,bForceImmediately=False,bNotifyUserSettings=False)"))

(event Custom|EndDialogSolved
  (EventDispatchers|BindEventtoOnEndText (stale Input|EnhancedActionEvents|EnhancedInputActionIA_Interact _output_get) (delegate Custom|EndText2)))

(event Custom|EndText2
  (bind _returnvalue (Game|GetPlayerController 0))
  (bind _returnvalue_2 (PlayerController|LocalPlayerSubsystems|GetEnhancedInputLocalPlayerSubsystem _returnvalue))
  (Widget|RemovefromParent (Variables|Default|GetTextbox))
  (Input|RemoveMappingContext _returnvalue_2 (Variables|Default|GetPuzzleMappingContext) "(bIgnoreAllPressedKeysUntilRelease=True,bForceImmediately=False,bNotifyUserSettings=False)")
  (Input|AddMappingContext _returnvalue_2 (Variables|Default|GetPlayerMappingContext) 0 "(bIgnoreAllPressedKeysUntilRelease=True,bForceImmediately=False,bNotifyUserSettings=False)"))

(event Input|EnhancedActionEvents|EnhancedInputActionIA_ExitPuzzle
  (params (ActionValue :type Boolean) (ElapsedSeconds :type Float%20%28double-precision%29) (TriggeredSeconds :type Float%20%28double-precision%29) (InputAction :type Input%20Action%20Object%20Reference :default "/Game/Inputs/InputActions/IA_ExitPuzzle.IA_ExitPuzzle"))
  (CallFunction|ReturntoCharacter))

(event Input|EnhancedActionEvents|EnhancedInputActionIA_Interact
  (params (ActionValue :type Boolean) (ElapsedSeconds :type Float%20%28double-precision%29) (TriggeredSeconds :type Float%20%28double-precision%29) (InputAction :type Input%20Action%20Object%20Reference :default "/Game/Inputs/InputActions/IA_Interact.IA_Interact"))
  (if (CallFunction|EvaluateCombination)
    (Input|RemoveMappingContext (PlayerController|LocalPlayerSubsystems|GetEnhancedInputLocalPlayerSubsystem (Game|GetPlayerController 0)) (Variables|Default|GetPuzzleMapping%20Context) "(bIgnoreAllPressedKeysUntilRelease=True,bForceImmediately=False,bNotifyUserSettings=False)")
    (CallFunction|SetSelectedWheelHighlight false)
    (Game|Player|SetViewTargetwithBlend (Game|GetPlayerController 0) (Variables|Default|GetCameraActor) (Variables|Default|GetSmoothPossessDuaration) "VTBlend_EaseInOut" (Variables|Default|GetPossessBlendExp) false)
    (Utilities|FlowControl|Delay (Variables|Default|GetSmoothPossessDuaration))
    (Audio|PlaySound2D 0 1.0 1.0 0.0 0 0)
    (bind _opendoor (Timeline|OpenSafe Play)
      (:Update
        (Transformation|SetRelativeRotation (Variables|Default|GetDoor) (Math|Rotator|MakeRotator 0.0 0.0 (* _opendoor (Variables|Default|GetOpenAngle))) false false)
        (Utilities|FlowControl|Delay 2.1)
        (CallFunction|ReturntoCharacter)
        (Variables|Default|SetCanBePossessed? false)
        (Variables|Default|SetAlreadyOpen true)))
    (else
      (Audio|PlaySound2D 0 1.0 1.0 0.0 0 0)
      (Input|RemoveMappingContext (PlayerController|LocalPlayerSubsystems|GetEnhancedInputLocalPlayerSubsystem (Game|GetPlayerController 0)) (Variables|Default|GetPuzzleMapping%20Context) "(bIgnoreAllPressedKeysUntilRelease=True,bForceImmediately=False,bNotifyUserSettings=False)")
      (bind _returnvalue (UserInterface|CreateWidget "/Game/UI/Textbox/WBP_Textbox.WBP_Textbox_C" 0 (Variables|Default|GetRow%20Number) (Variables|Default|GetData%20Table) (Variables|Default|GetEnd%20Of%20Row)))
      (bind _output_get (Variables|Default|SetTextbox _returnvalue))
      (UserInterface|Viewport|AddtoViewport _output_get 0)
      (EventDispatchers|BindEventtoOnEndText _output_get (delegate Custom|EndText)))))

(event Input|EnhancedActionEvents|EnhancedInputActionIA_NavigateRight
  (params (ActionValue :type Boolean) (ElapsedSeconds :type Float%20%28double-precision%29) (TriggeredSeconds :type Float%20%28double-precision%29) (InputAction :type Input%20Action%20Object%20Reference :default "/Game/Inputs/InputActions/IA_NavigateRight.IA_NavigateRight"))
  (Default|Rotate (Variables|Default|GetBP_SafeWheel) false))

(event Input|EnhancedActionEvents|EnhancedInputActionIA_NavigateLeft
  (params (ActionValue :type Boolean) (ElapsedSeconds :type Float%20%28double-precision%29) (TriggeredSeconds :type Float%20%28double-precision%29) (InputAction :type Input%20Action%20Object%20Reference :default "/Game/Inputs/InputActions/IA_NavigateLeft.IA_NavigateLeft"))
  (Default|Rotate (Variables|Default|GetBP_SafeWheel) true))

(event EventBeginPlay
  (|CallParentFunction))

(event EventReturntoCharacter
  (|CallParentFunction)
  (Variables|Default|SetSelectedRingIndex 0)
  (Widget|RemovefromParent (Variables|Default|GetRotatePuzzleWidget)))

(fn ConstructionScript)

(fn Interact
  (params (PlayerCharacter :type BP%20First%20Person%20Character%20Object%20Reference))
  (bind _returnvalue (Game|GetPlayerController 0))
  (bind _returnvalue_2 (PlayerController|LocalPlayerSubsystems|GetEnhancedInputLocalPlayerSubsystem _returnvalue))
  (|CallParentFunction PlayerCharacter)
  (if (Variables|Default|GetAlreadyOpen)
    (Input|AddMappingContext _returnvalue_2 (Variables|Default|GetPuzzleMapping%20Context) 0 "(bIgnoreAllPressedKeysUntilRelease=True,bForceImmediately=False,bNotifyUserSettings=False)")
    (Input|RemoveMappingContext _returnvalue_2 (Variables|Default|GetPlayerMappingContext) "(bIgnoreAllPressedKeysUntilRelease=True,bForceImmediately=False,bNotifyUserSettings=False)")
    (bind _returnvalue_3 (UserInterface|CreateWidget "/Game/UI/Textbox/WBP_Textbox.WBP_Textbox_C" 0 (Variables|Default|GetRow%20Number_0) (Variables|Default|GetData%20Table_0) (Variables|Default|GetEnd%20Of%20Row_0)))
    (bind _output_get (Variables|Default|SetTextbox _returnvalue_3))
    (UserInterface|Viewport|AddtoViewport _output_get 0)
    (CallFunction|EndDialogSolved)
    (return false)
    (else
      (CallFunction|SetSelectedWheelHighlight true)
      (bind _returnvalue_4 (UserInterface|CreateWidget "/Game/UI/PuzzlesUI/Controls/BPW_PuzzleControls.BPW_PuzzleControls_C" (Game|GetPlayerController 0) "" (Variables|Default|GetTexture)))
      (bind _output_get_2 (Variables|Default|SetRotatePuzzleWidget _returnvalue_4))
      (UserInterface|Viewport|AddtoViewport _output_get_2 0))))

(fn SetSelectedWheelHighlight
  (params (Enable :type Boolean))
  (CallFunction|SetHighlight Enable (Variables|Default|GetBP_SafeWheel)))

(fn GetSelectedWheel
  (return (Utilities|Array|Get(acopy) (Variables|Default|GetWheel) (Variables|Default|GetSelectedRingIndex))))

(fn EvaluateCombination
  (if (!= (Variables|Default|GetCorrectCode) (Variables|/Game/BP/SafePuzze/BP_SafeWheel.BP_SafeWheel_C|GetCurrentSelectedFace (Variables|Default|GetBP_SafeWheel)))
    (return false)
    (else
      (return true))))
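; Base interactable pawn that the player can possess, switching between first-person character control and puzzle controls.
; Interact stores the character and, if possession is allowed, starts the handover, while ReturnToCharacter reverses it.
; Both directions use either a camera fade or a timed view-target blend, swapping Enhanced Input mapping contexts and toggling the crosshair.
; SetHighlight toggles an outline on a given mesh through its overlay material.
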(event Custom|GetPossessed
  (Input|RemoveMappingContext (PlayerController|LocalPlayerSubsystems|GetEnhancedInputLocalPlayerSubsystem (Game|GetPlayerController 0)) (Variables|Default|GetPlayerMappingContext) "(bIgnoreAllPressedKeysUntilRelease=True,bForceImmediately=False,bNotifyUserSettings=False)")
  (if (Variables|Default|GetFade)
    (CameraFades|StartCameraFade :self (Game|GetPlayerCameraManager 0) :ToAlpha 1.0 :Duration (Variables|Default|GetFadeDuration) :bHoldWhenFinished true)
    (Utilities|FlowControl|Delay 2.0)
    (CameraFades|StartCameraFade :self (Game|GetPlayerCameraManager 0) :FromAlpha 1.0 :Duration (Variables|Default|GetFadeDuration))
    (else
      (Game|Player|SetViewTargetwithBlend (Game|GetPlayerController 0) self (Variables|Default|GetSmoothPossessDuration) (Variables|Default|GetPossessionBlendFunction) (Variables|Default|GetPossessBlendExponent) false)
      (Utilities|FlowControl|Delay (Variables|Default|GetSmoothPossessDuration))))
  (Pawn|Possess (Game|GetPlayerController 0) self)
  (Input|AddMappingContext (PlayerController|LocalPlayerSubsystems|GetEnhancedInputLocalPlayerSubsystem (Game|GetPlayerController 0)) (Variables|Default|GetPuzzleMappingContext) 0 "(bIgnoreAllPressedKeysUntilRelease=True,bForceImmediately=False,bNotifyUserSettings=False)")
  (Default|Show/HideCrosshair (Variables|Default|GetFirstPersonCharacter) false))

(event Custom|ReturnToCharacter
  (Input|RemoveMappingContext (PlayerController|LocalPlayerSubsystems|GetEnhancedInputLocalPlayerSubsystem (Game|GetPlayerController 0)) (Variables|Default|GetPuzzleMappingContext) "(bIgnoreAllPressedKeysUntilRelease=True,bForceImmediately=False,bNotifyUserSettings=False)")
  (if (Variables|Default|GetFade)
    (CameraFades|StartCameraFade :self (Game|GetPlayerCameraManager 0) :ToAlpha 1.0 :Duration (Variables|Default|GetFadeDuration) :bHoldWhenFinished true)
    (Utilities|FlowControl|Delay 2.0)
    (CameraFades|StartCameraFade :self (Game|GetPlayerCameraManager 0) :FromAlpha 1.0 :Duration (Variables|Default|GetFadeDuration))
    (else
      (Game|Player|SetViewTargetwithBlend (Game|GetPlayerController 0) (Variables|Default|GetFirstPersonCharacter) (Variables|Default|GetSmoothPossessDuration) (Variables|Default|GetPossessionBlendFunction) (Variables|Default|GetPossessBlendExponent) false)
      (Utilities|FlowControl|Delay (Variables|Default|GetSmoothPossessDuration))))
  (Input|AddMappingContext (PlayerController|LocalPlayerSubsystems|GetEnhancedInputLocalPlayerSubsystem (Game|GetPlayerController 0)) (Variables|Default|GetPlayerMappingContext) 0 "(bIgnoreAllPressedKeysUntilRelease=True,bForceImmediately=False,bNotifyUserSettings=False)")
  (Pawn|Possess (Game|GetPlayerController 0) (Variables|Default|GetFirstPersonCharacter))
  (Input|SetInputModeGameOnly (Game|GetPlayerController 0) false)
  (Default|Show/HideCrosshair (Variables|Default|GetFirstPersonCharacter) true))

(fn ConstructionScript)

(fn SetHighlight
  (params (Enable :type Boolean) (MeshComponent :type Mesh%20Component%20Object%20Reference))
  (Rendering|Material|SetOverlayMaterial MeshComponent (select Enable "/Game/Materials/Highlight/MM_Outline.MM_Outline" 0) :!class /Script/Engine.MeshComponent))

(fn Interact
  (params (PlayerCharacter :type BP%20First%20Person%20Character%20Object%20Reference))
  (Variables|Default|SetFirstPersonCharacter PlayerCharacter)
  (if (Variables|Default|GetCanBePossessed?)
    (CallFunction|GetPossessed)
    (return false)))
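; Collectable actor Blueprint that the player picks up by inspecting it, extending a parent's start and end inspection events.
; Starting inspection only runs the parent logic.
; Ending inspection calls the parent, sets Collected, toggles the Item component's visibility and destroys the actor.
; A second sequence branch then checks Collected, fires the OnCollect dispatcher after the destroy call and prints a debug string.
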(event EventBeginPlay
  (|CallParentFunction) ; This node is disabled and will not be called.\nDrag off pins to build functionality.
)

(event EventEndInspection
  (Utilities|FlowControl|Sequence
    (:then_0
      (|CallParentFunction)
      (Variables|Default|SetCollected true)
      (Rendering|ToggleVisibility (Variables|Default|GetItem) false)
      (Actor|DestroyActor))
    (:then_1
      (if (Variables|Default|GetCollected)
        (Default|CallOnCollect)
        (Development|PrintString "Call")))))

(event EventStartInspection
  (|CallParentFunction))

(fn ConstructionScript
  (|CallParentFunction))
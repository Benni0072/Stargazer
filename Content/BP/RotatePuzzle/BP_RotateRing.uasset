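; BP_RotateRing is a rotating puzzle ring that steps between numbered faces and reports the selected one as an enum value.
; Rotate moves the face index up or down, wraps it through ClampSelectedFace and converts it to a target yaw.
; Tick eases the relative rotation toward that yaw along the shortest path.
; The upper wrap triggers only above NumFaces, so an index equal to NumFaces passes through unchanged.
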(event Custom|Rotate
  (params (Up :type Boolean))
  (bind _output_get (Variables|Default|SetCurrentSelectedFace (CallFunction|ClampSelectedFace (+ (Variables|Default|GetCurrentSelectedFace) (Math|Integer|SelectInt 1 -1 Up)))))
  (Variables|Default|SetTargetRot (* (Math|Conversions|ToFloat(Integer) _output_get) (/ 3.6e+02 (Math|Conversions|ToFloat(Integer) (Variables|Default|GetNumFaces))) -1.0))
  (Development|PrintString (Utilities|String|ToString(Integer) (Variables|Default|GetCurrentSelectedFace))))

(event EventTick
  (params (DeltaSeconds :type Float%20%28single-precision%29))
  (Transformation|SetRelativeRotation (Math|Rotator|Lerp(Rotator) (Variables|Default|GetRelativeRotation) (Math|Rotator|MakeRotator 0.0 0.0 (Variables|Default|GetTargetRot)) (* (Utilities|Time|GetWorldDeltaSeconds) 1e+01) true) false false))

(fn GetCurrentNumber
  (return (Utilities|Select :Index (Variables|Default|GetCurrentSelectedFace) :Option%200 "NewEnumerator0" :Option%201 "NewEnumerator1" :Option%202 "NewEnumerator2" :Option%203 "NewEnumerator3" :Option%204 "NewEnumerator4" :Option%205 "NewEnumerator5" :Option%206 "NewEnumerator6" :Option%207 "NewEnumerator7" :Option%208 "NewEnumerator8")))

(fn ClampSelectedFace
  (params (Index :type Integer))
  (LocalVariables|SetClampeIndex Index)
  (Utilities|FlowControl|Sequence
    (:then_0
      (if (> (LocalVariables|GetClampeIndex) (Variables|Default|GetNumFaces))
        ;[0.15 0.15 0.15 0.5] if index greater than num facees, index - num faces. Ex: index 10 - num 9 = index 1 again
        (LocalVariables|SetClampeIndex (- (LocalVariables|GetClampeIndex) (Variables|Default|GetNumFaces)))))
    (:then_1
      (if (< (LocalVariables|GetClampeIndex) 0)
        ;[0.15 0.15 0.15 0.5] if index less than 0, add num faces to index. Ex.: index - 1 + num 9 = 8
        (LocalVariables|SetClampeIndex (+ (LocalVariables|GetClampeIndex) (Variables|Default|GetNumFaces)))))
    (:then_2
      (return (LocalVariables|GetClampeIndex)))))
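; Possessable three-ring combination puzzle that opens a door when the rings match the correct code.
; Navigation input selects a highlighted ring and rotates it, and Interact compares each ring's number to CorrectCode.
; Success locks the puzzle, blends to a camera, swings the door via Timeline, returns to the character and keeps scene components spinning on Tick.
; Failure shows a DataTable-driven textbox, suspending puzzle input until the text ends.
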(event Custom|EndText
  (Widget|RemovefromParent (Variables|Default|GetTextbox))
  (Input|AddMappingContext (PlayerController|LocalPlayerSubsystems|GetEnhancedInputLocalPlayerSubsystem (Game|GetPlayerController 0)) (Variables|Default|GetPuzzleMapping%20Context) 0 "(bIgnoreAllPressedKeysUntilRelease=True,bForceImmediately=False,bNotifyUserSettings=False)"))

(event Input|EnhancedActionEvents|EnhancedInputActionIA_ExitPuzzle
  (params (ActionValue :type Boolean) (ElapsedSeconds :type Float%20%28double-precision%29) (TriggeredSeconds :type Float%20%28double-precision%29) (InputAction :type Input%20Action%20Object%20Reference :default "/Game/Inputs/InputActions/IA_ExitPuzzle.IA_ExitPuzzle"))
  (CallFunction|ReturntoCharacter))

(event Input|EnhancedActionEvents|EnhancedInputActionIA_NavigateRight
  (params (ActionValue :type Boolean) (ElapsedSeconds :type Float%20%28double-precision%29) (TriggeredSeconds :type Float%20%28double-precision%29) (InputAction :type Input%20Action%20Object%20Reference :default "/Game/Inputs/InputActions/IA_NavigateRight.IA_NavigateRight"))
  (Default|Rotate (CallFunction|GetSelectedRing) false))

(event Input|EnhancedActionEvents|EnhancedInputActionIA_NavigateLeft
  (params (ActionValue :type Boolean) (ElapsedSeconds :type Float%20%28double-precision%29) (TriggeredSeconds :type Float%20%28double-precision%29) (InputAction :type Input%20Action%20Object%20Reference :default "/Game/Inputs/InputActions/IA_NavigateLeft.IA_NavigateLeft"))
  (Default|Rotate (CallFunction|GetSelectedRing) true))

(event Input|EnhancedActionEvents|EnhancedInputActionIA_NavigateUp
  (params (ActionValue :type Boolean) (ElapsedSeconds :type Float%20%28double-precision%29) (TriggeredSeconds :type Float%20%28double-precision%29) (InputAction :type Input%20Action%20Object%20Reference :default "/Game/Inputs/InputActions/IA_NavigateUp.IA_NavigateUp"))
  (CallFunction|ChangeSelectedRing true))

(event Input|EnhancedActionEvents|EnhancedInputActionIA_NavigateDown
  (params (ActionValue :type Boolean) (ElapsedSeconds :type Float%20%28double-precision%29) (TriggeredSeconds :type Float%20%28double-precision%29) (InputAction :type Input%20Action%20Object%20Reference :default "/Game/Inputs/InputActions/IA_NavigateDown.IA_NavigateDown"))
  (CallFunction|ChangeSelectedRing false))

(event Input|EnhancedActionEvents|EnhancedInputActionIA_Interact
  (params (ActionValue :type Boolean) (ElapsedSeconds :type Float%20%28double-precision%29) (TriggeredSeconds :type Float%20%28double-precision%29) (InputAction :type Input%20Action%20Object%20Reference :default "/Game/Inputs/InputActions/IA_Interact.IA_Interact"))
  (if (CallFunction|EvaluateCombination)
    (Audio|PlaySound2D 0 1.0 1.0 0.0 0 0)
    (Input|RemoveMappingContext (PlayerController|LocalPlayerSubsystems|GetEnhancedInputLocalPlayerSubsystem (Game|GetPlayerController 0)) (Variables|Default|GetPuzzleMapping%20Context) "(bIgnoreAllPressedKeysUntilRelease=True,bForceImmediately=False,bNotifyUserSettings=False)")
    (CallFunction|SetSelectetdRingHighlight false)
    (Variables|Default|SetSolvedPuzzle true)
    (Variables|Default|SetCanBePossessed? false)
    (Game|Player|SetViewTargetwithBlend (Game|GetPlayerController 0) (Variables|Default|GetCam) (Variables|Default|GetBlend%20Time) "VTBlend_EaseInOut" (Variables|Default|GetBlend%20Exp) false)
    (Utilities|FlowControl|Delay 1.0)
    (bind _opendoor (Timeline|Timeline Play)
      (:Update
        (Transformation|SetRelativeRotation (Variables|Default|GetDoor) (Math|Rotator|MakeRotator (* _opendoor (Variables|Default|GetOpenAngle)) 0.0 0.0) false false))
      (:Finished
        (Utilities|FlowControl|Delay 1.0)
        (CallFunction|ReturntoCharacter)))
    (else
      (Audio|PlaySound2D 0 1.0 1.0 0.0 0 0)
      (Input|RemoveMappingContext (PlayerController|LocalPlayerSubsystems|GetEnhancedInputLocalPlayerSubsystem (Game|GetPlayerController 0)) (Variables|Default|GetPuzzleMapping%20Context) "(bIgnoreAllPressedKeysUntilRelease=True,bForceImmediately=False,bNotifyUserSettings=False)")
      (bind _returnvalue (UserInterface|CreateWidget "/Game/UI/Textbox/WBP_Textbox.WBP_Textbox_C" 0 (Variables|Default|GetRow%20Number) (Variables|Default|GetData%20Table) (Variables|Default|GetEnd%20Of%20Row)))
      (bind _output_get (Variables|Default|SetTextbox _returnvalue))
      (UserInterface|Viewport|AddtoViewport _output_get 0)
      (EventDispatchers|BindEventtoOnEndText _output_get (delegate Custom|EndText)))))

(event EventBeginPlay
  (|CallParentFunction)
  (Variables|Default|SetRings (Utilities|Array|MakeArray (Variables|Default|GetBP_RotateRing) (Variables|Default|GetBP_RotateRing1) (Variables|Default|GetBP_RotateRing2))))

(event EventTick
  (params (DeltaSeconds :type Float%20%28single-precision%29))
  (if (Variables|Default|GetSolvedPuzzle)
    (Transformation|AddRelativeRotation (Variables|Default|GetScene) (Math|Rotator|MakeRotator 0.0 0.0 (* (Variables|Default|GetAnimationSpeed) (Utilities|Time|GetWorldDeltaSeconds))) false false)
    (Transformation|AddRelativeRotation (Variables|Default|GetScene2) (Math|Rotator|MakeRotator 0.0 0.0 (* 2e+01 (Utilities|Time|GetWorldDeltaSeconds))) false false)
    (Transformation|AddRelativeRotation (Variables|Default|GetScene3) (Math|Rotator|MakeRotator 0.0 0.0 (* 3e+01 (Utilities|Time|GetWorldDeltaSeconds))) false false)))

(event EventReturntoCharacter
  (|CallParentFunction)
  (Variables|Default|SetSelectedRingIndex 0)
  (Widget|RemovefromParent (Variables|Default|GetControlWidget)))

(fn ConstructionScript)

(fn Interact
  (params (PlayerCharacter :type BP%20First%20Person%20Character%20Object%20Reference))
  (|CallParentFunction PlayerCharacter)
  (if (Variables|Default|GetSolvedPuzzle)
    (CallFunction|SetSelectetdRingHighlight false)
    (return false)
    (else
      (CallFunction|SetSelectetdRingHighlight true)
      (bind _returnvalue (UserInterface|CreateWidget "/Game/UI/PuzzlesUI/Controls/BPW_PuzzleControls.BPW_PuzzleControls_C" (Game|GetPlayerController 0) (Variables|Default|GetControllText)))
      (bind _output_get (Variables|Default|SetControlWidget _returnvalue))
      (UserInterface|Viewport|AddtoViewport _output_get 0))))

(fn SetSelectetdRingHighlight
  (params (Enable :type Boolean))
  (CallFunction|SetHighlight Enable (CallFunction|GetSelectedRing)))

(fn GetSelectedRing
  (return (Utilities|Array|Get(acopy) (Variables|Default|GetRings) (Variables|Default|GetSelectedRingIndex))))

(fn ChangeSelectedRing
  (params (Right :type Boolean))
  (CallFunction|SetSelectetdRingHighlight false)
  (Variables|Default|SetSelectedRingIndex (Math|Integer|Clamp(Integer) (+ (Variables|Default|GetSelectedRingIndex) (Math|Integer|SelectInt 1 -1 Right)) 0 (Utilities|Array|LastIndex (Variables|Default|GetRings))))
  (CallFunction|SetSelectetdRingHighlight true))

(fn EvaluateCombination
  (for (_array_element _array_index) (Variables|Default|GetRings)
    (if (Utilities|Enum|NotEqual(Enum) (Default|GetCurrentNumber _array_element) (Utilities|Array|Get(acopy) (Variables|Default|GetCorrectCode) _array_index))
      (return false)))
  (return true))
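; BP_EndTrigger is an interactable that becomes possessable only after its linked Stardust is collected.
; The Stardust's collect event sets HasStardust and updates CanBePossessed, currently its only real condition.
; Interact calls the parent, then, if not possessable, removes the player's input mapping context and shows a data-table-driven WBP_Textbox.
; The textbox receives a self reference, and EndText restores the mapping context and removes the widget.
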(event Custom|OnCollected_Event
  (Variables|Default|SetHasStardust true)
  (CallFunction|UpdateCanbePossessed))

(event Custom|EndText
  (Input|AddMappingContext (PlayerController|LocalPlayerSubsystems|GetEnhancedInputLocalPlayerSubsystem (Game|GetPlayerController 0)) (Variables|Default|GetPlayerMappingContext) 0 "(bIgnoreAllPressedKeysUntilRelease=True,bForceImmediately=False,bNotifyUserSettings=False)")
  (Widget|RemovefromParent (Variables|Default|GetNotPossessableWidget)))

(event EventBeginPlay
  (EventDispatchers|BindEventtoOnCollect (Variables|Default|GetStardust) (delegate Custom|OnCollected_Event)))

(fn ConstructionScript)

(fn Interact
  (params (PlayerCharacter :type BP%20First%20Person%20Character%20Object%20Reference))
  (|CallParentFunction PlayerCharacter)
  (if (Variables|Default|GetCanBePossessed?)
    (return false)
    (else
      (Input|RemoveMappingContext (PlayerController|LocalPlayerSubsystems|GetEnhancedInputLocalPlayerSubsystem (Game|GetPlayerController 0)) (Variables|Default|GetPlayerMappingContext) "(bIgnoreAllPressedKeysUntilRelease=True,bForceImmediately=False,bNotifyUserSettings=False)")
      (bind _returnvalue (UserInterface|CreateWidget "/Game/UI/Textbox/WBP_Textbox.WBP_Textbox_C" 0 (Variables|Default|GetNotPosessableRow%20Number) (Variables|Default|GetNotPossessableData%20Table) (Variables|Default|GetNotPossessableEnd%20Of%20Row)))
      (bind _output_get (Variables|Default|SetNotPossessableWidget _returnvalue))
      (Variables|/Game/UI/Textbox/WBP_Textbox.WBP_Textbox_C|SetEndTrigger _returnvalue self)
      (UserInterface|Viewport|AddtoViewport _output_get 0))))

(fn UpdateCanbePossessed
  (Variables|Default|SetCanBePossessed? (and (Variables|Default|GetHasStardust) true)))
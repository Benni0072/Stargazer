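; Jellyfish actor Blueprint that animates its Sphere component's vertical position.
; On BeginPlay, the Hight flag selects one of two timelines, Jellyfish or Timeline.
; Each timeline's Updown track, scaled by Speed, sets the sphere's relative Z location on every update.
; Speed multiplies the offset, so it controls travel distance rather than playback rate.
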(event EventBeginPlay
  (if (Variables|Default|GetHight)
    (bind _updown (Timeline|Jellyfish Play)
      (:Update
        (Transformation|SetRelativeLocation (Variables|Default|GetSphere) (Math|Vector|MakeVector 0.0 0.0 (* _updown (Variables|Default|GetSpeed))) false false)))
    (else
      (bind _updown_2 (Timeline|Timeline Play)
        (:Update
          (Transformation|SetRelativeLocation (Variables|Default|GetSphere) (Math|Vector|MakeVector 0.0 0.0 (* _updown_2 (Variables|Default|GetSpeed))) false false))))))

(fn ConstructionScript)
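; BP_Planets is an actor that continuously spins three static mesh components around their yaw axis, apparently as animated planets.
; On Tick, each mesh gets a relative rotation scaled by world delta seconds, so the spin is frame-rate independent.
; The first mesh uses the AnimationSpeed variable, while the other two turn at fixed, different rates.
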(event EventBeginPlay)

(event EventTick
  (params (DeltaSeconds :type Float%20%28single-precision%29))
  (Transformation|AddRelativeRotation (Variables|Default|GetStaticMesh) (Math|Rotator|MakeRotator 0.0 0.0 (* (Variables|Default|GetAnimationSpeed) (Utilities|Time|GetWorldDeltaSeconds))) false false)
  (Transformation|AddRelativeRotation (Variables|Default|GetStaticMesh1) (Math|Rotator|MakeRotator 0.0 0.0 (* 4.0 (Utilities|Time|GetWorldDeltaSeconds))) false false)
  (Transformation|AddRelativeRotation (Variables|Default|GetStaticMesh2) (Math|Rotator|MakeRotator 0.0 0.0 (* 6.0 (Utilities|Time|GetWorldDeltaSeconds))) false false))

(event Collision|EventActorBeginOverlap
  (params (OtherActor :type Actor%20Object%20Reference)))

(fn ConstructionScript)
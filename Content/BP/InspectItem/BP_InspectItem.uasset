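; BP_InspectItem is an inspectable item that shows a text box while the first-person character inspects it.
; BeginPlay caches the item's starting transform and the player character.
; StartInspection creates a WBP_Textbox fed by a data table, start row and end row, and gives it a back-reference to the item.
; EndInspection clears the character's InspectItem, restores the original transform and removes the widget.
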(event Custom|StartInspection
  (bind _returnvalue (UserInterface|CreateWidget "/Game/UI/Textbox/WBP_Textbox.WBP_Textbox_C" (Game|GetPlayerController 0) (Variables|Default|GetRow%20Number) (Variables|Default|GetData%20Table) (Variables|Default|GetEnd%20Of%20Row)))
  (bind _output_get (Variables|Default|SetTextboxWidget _returnvalue))
  (Variables|/Game/UI/Textbox/WBP_Textbox.WBP_Textbox_C|SetBP%20Inspect%20Item _output_get self)
  (UserInterface|Viewport|AddtoViewport _output_get 0))

(event Custom|EndInspection
  (Variables|/Game/BP/BP_FirstPersonCharacter.BP_FirstPersonCharacter_C|SetInspectItem (Variables|Default|GetAs%20BP%20First%20Person%20Character) 0)
  (Transformation|SetActorTransform (Variables|Default|GetStartTransform))
  (Widget|RemovefromParent (Variables|Default|GetTextboxWidget)))

(event EventBeginPlay
  (Variables|Default|SetStartTransform (Transformation|GetActorTransform))
  (bind _asbp_first_person_character (Utilities|Casting|CastToBP_FirstPersonCharacter (Game|GetPlayerCharacter 0)))
  (Variables|Default|SetAs%20BP%20First%20Person%20Character _asbp_first_person_character))

(fn ConstructionScript)
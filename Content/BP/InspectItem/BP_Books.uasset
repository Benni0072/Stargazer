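; BP_Books is an interactable book that opens a zodiac sign book widget on screen.
; Interact, when the book is not already open, swaps the player input mapping context for the puzzle one, then creates and shows BPW_ZodiacSignBook.
; The widget's end-text callback removes it, restores player input and clears the Open flag so the book can be used again.
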(event Custom|CreateWidget
  (Input|RemoveMappingContext (PlayerController|LocalPlayerSubsystems|GetEnhancedInputLocalPlayerSubsystem (Game|GetPlayerController 0)) (Variables|Default|GetPlayerMappingContext) "(bIgnoreAllPressedKeysUntilRelease=True,bForceImmediately=False,bNotifyUserSettings=False)")
  (Input|AddMappingContext (PlayerController|LocalPlayerSubsystems|GetEnhancedInputLocalPlayerSubsystem (Game|GetPlayerController 0)) (Variables|Default|GetPuzzleMappingContext) 0 "(bIgnoreAllPressedKeysUntilRelease=True,bForceImmediately=False,bNotifyUserSettings=False)")
  (bind _returnvalue (UserInterface|CreateWidget "/Game/UI/PuzzlesUI/Books/BPW_ZodiacSignBook.BPW_ZodiacSignBook_C" (Game|GetPlayerController 0)))
  (bind _output_get (Variables|Default|SetZodiacSignBook _returnvalue))
  (UserInterface|Viewport|AddtoViewport _output_get 0)
  (if (not (Variables|Default|GetOpen?))
    (Variables|Default|SetOpen? true)
    (EventDispatchers|BindEventtoEndText (Variables|Default|GetZodiacSignBook) (delegate Custom|EndWidget))))

(event Custom|EndWidget
  (Input|RemoveMappingContext (PlayerController|LocalPlayerSubsystems|GetEnhancedInputLocalPlayerSubsystem (Game|GetPlayerController 0)) (Variables|Default|GetPuzzleMappingContext) "(bIgnoreAllPressedKeysUntilRelease=True,bForceImmediately=False,bNotifyUserSettings=False)")
  (Input|AddMappingContext (PlayerController|LocalPlayerSubsystems|GetEnhancedInputLocalPlayerSubsystem (Game|GetPlayerController 0)) (Variables|Default|GetPlayerMappingContext) 0 "(bIgnoreAllPressedKeysUntilRelease=True,bForceImmediately=False,bNotifyUserSettings=False)")
  (Widget|RemovefromParent (Variables|Default|GetZodiacSignBook))
  (Variables|Default|SetOpen? false))

(fn ConstructionScript)

(fn Interact
  (params (PlayerCharacter :type BP%20First%20Person%20Character%20Object%20Reference))
  (if (not (Variables|Default|GetOpen?))
    (CallFunction|CreateWidget)
    (return false)))
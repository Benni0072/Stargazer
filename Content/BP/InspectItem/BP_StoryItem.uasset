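; BP_StoryItem is an interactable item that shows text in a textbox widget when the player interacts with it.
; Interact creates a WBP_Textbox, passing it the DataTable, RowNumber, EndOfRow and a reference to the item, then returns false.
; The player mapping context is removed while the textbox is open.
; The widget's OnEndText event restores that context and removes the textbox.
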(event Custom|CreateWidget
  (Input|RemoveMappingContext (PlayerController|LocalPlayerSubsystems|GetEnhancedInputLocalPlayerSubsystem (Game|GetPlayerController 0)) (Variables|Default|GetPlayerMappingContext) "(bIgnoreAllPressedKeysUntilRelease=True,bForceImmediately=False,bNotifyUserSettings=False)")
  (bind _returnvalue (UserInterface|CreateWidget "/Game/UI/Textbox/WBP_Textbox.WBP_Textbox_C" (Game|GetPlayerController 0) (Variables|Default|GetRow%20Number) (Variables|Default|GetData%20Table) (Variables|Default|GetEnd%20Of%20Row)))
  (bind _output_get (Variables|Default|SetTextboxWidget _returnvalue))
  (Variables|/Game/UI/Textbox/WBP_Textbox.WBP_Textbox_C|SetStoryItem _returnvalue self)
  (UserInterface|Viewport|AddtoViewport _output_get 0)
  (EventDispatchers|BindEventtoOnEndText (Variables|Default|GetTextboxWidget) (delegate Custom|EndText)))

(event Custom|EndText
  (Input|AddMappingContext (PlayerController|LocalPlayerSubsystems|GetEnhancedInputLocalPlayerSubsystem (Game|GetPlayerController 0)) (Variables|Default|GetPlayerMappingContext) 0 "(bIgnoreAllPressedKeysUntilRelease=True,bForceImmediately=False,bNotifyUserSettings=False)")
  (Widget|RemovefromParent (Variables|Default|GetTextboxWidget)))

(fn ConstructionScript)

(fn Interact
  (params (PlayerCharacter :type BP%20First%20Person%20Character%20Object%20Reference))
  (CallFunction|CreateWidget)
  (return false))
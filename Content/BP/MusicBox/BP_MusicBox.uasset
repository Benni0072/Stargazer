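; Music box puzzle: the player rotates the top to a face and confirms it against the correct code.
; Interacting shows the controls widget and highlight, or only a textbox once solved; a wrong answer shows a textbox while puzzle input is suspended.
; Solving starts a whale-bobbing timeline and Tick-driven spinning, plays music, returns to the character, shows the middle comic, disables possession and closes the curtain.
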(event Custom|EndDialogSolvedText
  (Widget|RemovefromParent (Variables|Default|GetTextbox)))

(event Custom|EndDialog
  (params (Target :type WBP%20Textbox%20Object%20Reference))
  (EventDispatchers|BindEventtoOnEndText Target (delegate Custom|EndDialogSolvedText)))

(event Custom|EndText
  (Widget|RemovefromParent (Variables|Default|GetTextbox))
  (Input|AddMappingContext (PlayerController|LocalPlayerSubsystems|GetEnhancedInputLocalPlayerSubsystem (Game|GetPlayerController 0)) (Variables|Default|GetPuzzleMapping%20Context) 0 "(bIgnoreAllPressedKeysUntilRelease=True,bForceImmediately=False,bNotifyUserSettings=False)"))

(event Input|EnhancedActionEvents|EnhancedInputActionIA_ExitPuzzle
  (params (ActionValue :type Boolean) (ElapsedSeconds :type Float%20%28double-precision%29) (TriggeredSeconds :type Float%20%28double-precision%29) (InputAction :type Input%20Action%20Object%20Reference :default "/Game/Inputs/InputActions/IA_ExitPuzzle.IA_ExitPuzzle"))
  (CallFunction|ReturntoCharacter))

(event Input|EnhancedActionEvents|EnhancedInputActionIA_NavigateLeft
  (params (ActionValue :type Boolean) (ElapsedSeconds :type Float%20%28double-precision%29) (TriggeredSeconds :type Float%20%28double-precision%29) (InputAction :type Input%20Action%20Object%20Reference :default "/Game/Inputs/InputActions/IA_NavigateLeft.IA_NavigateLeft"))
  (Default|Rotation (Variables|Default|GetBP_MusicboxTop) false)
  (Audio|PlaySound2D "/Game/Sound/SFX/Musicbox/Musicbox.Musicbox" 1.0 1.0 0.0 0 0))

(event Input|EnhancedActionEvents|EnhancedInputActionIA_Interact
  (params (ActionValue :type Boolean) (ElapsedSeconds :type Float%20%28double-precision%29) (TriggeredSeconds :type Float%20%28double-precision%29) (InputAction :type Input%20Action%20Object%20Reference :default "/Game/Inputs/InputActions/IA_Interact.IA_Interact"))
  (bind _whale1 (Variables|Default|GetWhale1))
  (bind _whale2 (Variables|Default|GetWhale2))
  (bind _relativelocation (Variables|/Script/Engine.SceneComponent|GetRelativeLocation _whale1))
  (bind _relativelocation_2 (Variables|/Script/Engine.SceneComponent|GetRelativeLocation _whale2))
  (if (CallFunction|EvaluateCombination)
    (Input|RemoveMappingContext (PlayerController|LocalPlayerSubsystems|GetEnhancedInputLocalPlayerSubsystem (Game|GetPlayerController 0)) (Variables|Default|GetPuzzleMapping%20Context) "(bIgnoreAllPressedKeysUntilRelease=True,bForceImmediately=False,bNotifyUserSettings=False)")
    (CallFunction|SetSelectedWheelHighlight false)
    (Variables|Default|SetPuzzleSolved true)
    (bind (_direction _updownwhale1 _updownwhale2) (Timeline|MusicBox Play)
      (:Update
        (Transformation|SetRelativeLocation _whale1 (Math|Vector|MakeVector (.x _relativelocation) (.y _relativelocation) (Math|Float|Lerp (Variables|Default|GetStartPosition) (+ (Variables|Default|GetStartPosition) 0.8) _updownwhale1)) false false)
        (Transformation|SetRelativeLocation _whale2 (Math|Vector|MakeVector (.x _relativelocation_2) (.y _relativelocation_2) (Math|Float|Lerp (Variables|Default|GetStartPosition) (+ (Variables|Default|GetStartPosition) 0.8) _updownwhale2)) false false)
        (Utilities|FlowControl|DoOnce false
          (:Completed
            (Audio|PlaySound2D "/Game/Sound/Music/LonelyGalaxy.LonelyGalaxy" 1.0 1.0 0.0 0 0)
            (Utilities|FlowControl|Delay 1.0)
            (CallFunction|ReturntoCharacter)
            (Utilities|FlowControl|Delay 1.0)
            (bind _returnvalue (UserInterface|CreateWidget "/Game/UI/Comics/MiddleComic/BPW_MiddleComic.BPW_MiddleComic_C" (Game|GetPlayerController 0)))
            (bind _output_get (Variables|Default|SetMiddleComic _returnvalue))
            (UserInterface|Viewport|AddtoViewport _output_get 0)
            (Variables|Default|SetCanBePossessed? false)
            (Components|StaticMesh|SetStaticMesh (Variables|/Script/Engine.StaticMeshActor|GetStaticMeshComponent (Variables|Default|GetCurtain)) "/Game/Assets/Curtains/CurtainClosed.CurtainClosed")))))
    (else
      (Input|RemoveMappingContext (PlayerController|LocalPlayerSubsystems|GetEnhancedInputLocalPlayerSubsystem (Game|GetPlayerController 0)) (Variables|Default|GetPuzzleMapping%20Context) "(bIgnoreAllPressedKeysUntilRelease=True,bForceImmediately=False,bNotifyUserSettings=False)")
      (bind _returnvalue_2 (UserInterface|CreateWidget "/Game/UI/Textbox/WBP_Textbox.WBP_Textbox_C" 0 (Variables|Default|GetRow%20Number) (Variables|Default|GetData%20Table) (Variables|Default|GetEnd%20Of%20Row)))
      (bind _output_get_2 (Variables|Default|SetTextbox _returnvalue_2))
      (UserInterface|Viewport|AddtoViewport _output_get_2 0)
      (EventDispatchers|BindEventtoOnEndText _output_get_2 (delegate Custom|EndText)))))

(event EventBeginPlay
  (|CallParentFunction))

(event EventReturntoCharacter
  (|CallParentFunction)
  (Variables|Default|SetSelectedRingIndex 0)
  (Widget|RemovefromParent (Variables|Default|GetControlWidget)))

(event EventTick
  (params (DeltaSeconds :type Float%20%28single-precision%29))
  (if (Variables|Default|GetPuzzleSolved)
    (Transformation|AddRelativeRotation (Variables|Default|GetMusicboxTopPart) (Math|Rotator|MakeRotator 0.0 0.0 (* (Variables|Default|GetAnimationSpeed) (Utilities|Time|GetWorldDeltaSeconds))) false false)
    (Transformation|AddRelativeRotation (Variables|Default|GetPlane_013) (Math|Rotator|MakeRotator (* (Variables|Default|GetAnimationSpeed) (Utilities|Time|GetWorldDeltaSeconds)) 0.0 0.0) false false)))

(fn ConstructionScript)

(fn SetSelectedWheelHighlight
  (params (Enable :type Boolean))
  (CallFunction|SetHighlight Enable (Variables|Default|GetBP_MusicboxTop)))

(fn Interact
  (params (PlayerCharacter :type BP%20First%20Person%20Character%20Object%20Reference))
  (|CallParentFunction PlayerCharacter)
  (if (Variables|Default|GetPuzzleSolved)
    (CallFunction|SetSelectedWheelHighlight false)
    (bind _returnvalue (UserInterface|CreateWidget "/Game/UI/Textbox/WBP_Textbox.WBP_Textbox_C" 0 (Variables|Default|GetRow%20Number_0) (Variables|Default|GetData%20Table_0) (Variables|Default|GetEnd%20Of%20Row_0)))
    (bind _output_get (Variables|Default|SetTextboxWidget _returnvalue))
    (UserInterface|Viewport|AddtoViewport _output_get 0)
    (Default|Show/HideCrosshair (Variables|Default|GetAs%20BP%20First%20Person%20Character) false)
    (CallFunction|EndDialog _output_get)
    (return false)
    (else
      (CallFunction|SetSelectedWheelHighlight true)
      (bind _returnvalue_2 (UserInterface|CreateWidget "/Game/UI/PuzzlesUI/Controls/BPW_PuzzleControls.BPW_PuzzleControls_C" 0 (Variables|Default|GetControllText)))
      (bind _output_get_2 (Variables|Default|SetControlWidget _returnvalue_2))
      (UserInterface|Viewport|AddtoViewport _output_get_2 0)
      (return false))))

(fn EvaluateCombination
  (if (!= (Variables|Default|GetCorrectCode) (Variables|/Game/BP/MusicBox/BP_MusicboxTop.BP_MusicboxTop_C|GetCurrentSelectedFace (Variables|Default|GetBP_MusicboxTop)))
    (return false)
    (else
      (return true))))
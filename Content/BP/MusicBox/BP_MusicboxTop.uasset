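; BP_MusicboxTop is the rotating top of a music box, stepped between evenly spaced faces.
; Rotation moves the selected face index up or down, wraps it within the face count and derives a negated target yaw.
; Tick eases the relative rotation toward that yaw along the shortest path.
; GetCurrentNumber returns one of four enum values, indexed by the face count rather than the selected face.
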(event Custom|Rotation
  (params (Up :type Boolean))
  (bind _output_get (Variables|Default|SetCurrentSelectedFace (CallFunction|ClampSelectedFace (+ (Variables|Default|GetCurrentSelectedFace) (Math|Integer|SelectInt 1 -1 Up)))))
  (Variables|Default|SetTargetRot (* (Math|Conversions|ToFloat(Integer) _output_get) (/ 3.6e+02 (Math|Conversions|ToFloat(Integer) (Variables|Default|GetNumFaces))) -1.0)))

(event EventTick
  (params (DeltaSeconds :type Float%20%28single-precision%29))
  (Transformation|SetRelativeRotation (Math|Rotator|Lerp(Rotator) (Variables|Default|GetRelativeRotation) (Math|Rotator|MakeRotator 0.0 0.0 (Variables|Default|GetTargetRot)) (* (Utilities|Time|GetWorldDeltaSeconds) 1e+01) true) false false))

(fn ClampSelectedFace
  (params (Index :type Integer))
  (LocalVariables|SetClampeIndex Index)
  (Utilities|FlowControl|Sequence
    (:then_0
      (if (> (LocalVariables|GetClampeIndex) (- (Variables|Default|GetNumFaces) 1))
        (LocalVariables|SetClampeIndex (- (LocalVariables|GetClampeIndex) (Variables|Default|GetNumFaces)))))
    (:then_1
      (if (< (LocalVariables|GetClampeIndex) 0)
        (LocalVariables|SetClampeIndex (+ (LocalVariables|GetClampeIndex) (Variables|Default|GetNumFaces)))))
    (:then_2
      (return (LocalVariables|GetClampeIndex)))))

(fn GetCurrentNumber
  (return (Utilities|Select :Index (Variables|Default|GetNumFaces) :Option%200 "NewEnumerator0" :Option%201 "NewEnumerator1" :Option%202 "NewEnumerator2" :Option%203 "NewEnumerator3")))
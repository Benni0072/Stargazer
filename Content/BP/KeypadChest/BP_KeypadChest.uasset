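; BP_KeypadChest is an interactable chest Blueprint with a set of keypad buttons, one of which is selected at a time.
; Interact calls the parent implementation, highlights the selected button and always returns false.
; The highlight sets an overlay material on the button found at CurrentButtonIndex in the Buttons array, switched by an Enable flag.
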(fn ConstructionScript)

(fn Interact
  (params (PlayerCharacter :type BP%20First%20Person%20Character%20Object%20Reference))
  (|CallParentFunction PlayerCharacter)
  (CallFunction|UpdateHighlightOfSelectedButton true)
  (return false))

(fn UpdateHighlightOfSelectedButton
  (params (Enable :type Boolean))
  (Rendering|Material|SetOverlayMaterial (CallFunction|GetSelectedButton) (select Enable 0 0) :!class /Script/Engine.MeshComponent))

(fn GetSelectedButton
  (return (Utilities|Array|Get(acopy) (Variables|Default|GetButtons) (Variables|Default|GetCurrentButtonIndex))))
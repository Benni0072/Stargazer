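; BP_RotationDisc is a rotating disc for the star puzzle, with numbered faces and a selected face exposed as an enum through GetCurrentNumber.
; Rotate converts the selected face into a target yaw, and Tick eases toward it by shortest-path lerp.
; The ClampSelectedFace step-down call never executes, so Rotate reads its unset output.
; That function's underflow wraps to NumFaces, one past the last index.
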(event Custom|Rotate
  (bind _output_get (Variables|Default|SetCurrentSelectedFace (stale _returnvalue)))
  (Variables|Default|SetTargetRot (* (Math|Conversions|ToFloat(Integer) _output_get) (/ 3.6e+02 (Math|Conversions|ToFloat(Integer) (Variables|Default|GetNumFaces))) -1.0)))

(event EventTick
  (params (DeltaSeconds :type Float%20%28single-precision%29))
  (Transformation|SetRelativeRotation (Math|Rotator|Lerp(Rotator) (Variables|Default|GetRelativeRotation) (Math|Rotator|MakeRotator 0.0 0.0 (Variables|Default|GetTargetRot)) (* (Utilities|Time|GetWorldDeltaSeconds) 1e+01) true) false false))

(fn GetCurrentNumber
  (return (Utilities|Select :Index (Variables|Default|GetCurrentSelectedFace) :Option%200 "NewEnumerator0" :Option%201 "NewEnumerator1" :Option%202 "NewEnumerator2" :Option%203 "NewEnumerator3" :Option%204 "NewEnumerator4" :Option%205 "NewEnumerator5" :Option%206 "NewEnumerator6" :Option%207 "NewEnumerator7" :Option%208 "NewEnumerator8")))

(fn ClampSelectedFace
  (params (Index :type Integer))
  (LocalVariables|SetClampeIndex Index)
  (Utilities|FlowControl|Sequence
    (:then_0
      (if (> (LocalVariables|GetClampeIndex) (- (Variables|Default|GetNumFaces) 1))
        (LocalVariables|SetClampeIndex 0)))
    (:then_1
      (if (< (LocalVariables|GetClampeIndex) 0)
        (LocalVariables|SetClampeIndex (- (Variables|Default|GetNumFaces) 0))))
    (:then_2
      (return (LocalVariables|GetClampeIndex)))))
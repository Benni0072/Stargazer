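; Possessable star puzzle where the player rotates three discs to match a code and open a door.
; Input actions move a highlight between discs and rotate the selected one, with a fading widget overlay.
; Interact checks each disc against CorrectCode: failure shows a textbox and suspends puzzle input until it ends.
; Success animates zodiac material emission, switches camera, swings the door open via timeline, marks the puzzle solved and returns to the character.
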(event Custom|EndText
  (Widget|RemovefromParent (Variables|Default|GetTextbox))
  (Input|AddMappingContext (PlayerController|LocalPlayerSubsystems|GetEnhancedInputLocalPlayerSubsystem (Game|GetPlayerController 0)) (Variables|Default|GetPuzzleMapping%20Context) 0 "(bIgnoreAllPressedKeysUntilRelease=True,bForceImmediately=False,bNotifyUserSettings=False)"))

(event Custom|EmissionAnimation
  (bind _heart (Timeline|Timeline Play)
    (:Update
      (Rendering|Material|SetScalarParameterValue (Variables|Default|GetMID) "Emission" _heart :!class /Script/Engine.MaterialInstanceDynamic))))

(event Custom|Delay
  (Utilities|FlowControl|Delay 2.0)
  (bind _returnvalue (UserInterface|CreateWidget "/Game/BP/StarPuzzle/WBP_StarRotatePuzzle.WBP_StarRotatePuzzle_C" (Game|GetPlayerController 0)))
  (bind _output_get (Variables|Default|SetWBP_StarRotatePuzzle _returnvalue))
  (UserInterface|Viewport|AddtoViewport _output_get 0)
  (UserInterface|Animation|PlayAnimation _output_get (Variables|/Game/BP/StarPuzzle/WBP_StarRotatePuzzle.WBP_StarRotatePuzzle_C|GetFadeInOut _output_get) 0.0 1 "Forward" 1.0 false))

(event Input|EnhancedActionEvents|EnhancedInputActionIA_ExitPuzzle
  (params (ActionValue :type Boolean) (ElapsedSeconds :type Float%20%28double-precision%29) (TriggeredSeconds :type Float%20%28double-precision%29) (InputAction :type Input%20Action%20Object%20Reference :default "/Game/Inputs/InputActions/IA_ExitPuzzle.IA_ExitPuzzle"))
  (bind _wbp_starrotatepuzzle (Variables|Default|GetWBP_StarRotatePuzzle))
  (UserInterface|Animation|PlayAnimation _wbp_starrotatepuzzle (Variables|/Game/BP/StarPuzzle/WBP_StarRotatePuzzle.WBP_StarRotatePuzzle_C|GetFadeInOut _wbp_starrotatepuzzle) 0.0 1 "Reverse" 1.0 false)
  (CallFunction|ReturntoCharacter)
  (Utilities|FlowControl|Delay 1.0)
  (Widget|RemovefromParent _wbp_starrotatepuzzle))

(event Input|EnhancedActionEvents|EnhancedInputActionIA_NavigateRight
  (params (ActionValue :type Boolean) (ElapsedSeconds :type Float%20%28double-precision%29) (TriggeredSeconds :type Float%20%28double-precision%29) (InputAction :type Input%20Action%20Object%20Reference :default "/Game/Inputs/InputActions/IA_NavigateRight.IA_NavigateRight"))
  (CallFunction|ChangeSelectedDisc true))

(event Input|EnhancedActionEvents|EnhancedInputActionIA_NavigateLeft
  (params (ActionValue :type Boolean) (ElapsedSeconds :type Float%20%28double-precision%29) (TriggeredSeconds :type Float%20%28double-precision%29) (InputAction :type Input%20Action%20Object%20Reference :default "/Game/Inputs/InputActions/IA_NavigateLeft.IA_NavigateLeft"))
  (CallFunction|ChangeSelectedDisc false))

(event Input|EnhancedActionEvents|EnhancedInputActionIA_NavigateUp
  (params (ActionValue :type Boolean) (ElapsedSeconds :type Float%20%28double-precision%29) (TriggeredSeconds :type Float%20%28double-precision%29) (InputAction :type Input%20Action%20Object%20Reference :default "/Game/Inputs/InputActions/IA_NavigateUp.IA_NavigateUp"))
  (Default|Rotate (CallFunction|GetSelectedDisc) false))

(event Input|EnhancedActionEvents|EnhancedInputActionIA_NavigateDown
  (params (ActionValue :type Boolean) (ElapsedSeconds :type Float%20%28double-precision%29) (TriggeredSeconds :type Float%20%28double-precision%29) (InputAction :type Input%20Action%20Object%20Reference :default "/Game/Inputs/InputActions/IA_NavigateDown.IA_NavigateDown"))
  (Default|Rotate (CallFunction|GetSelectedDisc) true))

(event Input|EnhancedActionEvents|EnhancedInputActionIA_Interact
  (params (ActionValue :type Boolean) (ElapsedSeconds :type Float%20%28double-precision%29) (TriggeredSeconds :type Float%20%28double-precision%29) (InputAction :type Input%20Action%20Object%20Reference :default "/Game/Inputs/InputActions/IA_Interact.IA_Interact"))
  (bind _wbp_starrotatepuzzle (Variables|Default|GetWBP_StarRotatePuzzle))
  (if (CallFunction|EvaluateCombination)
    (Audio|PlaySound2D 0 1.0 1.0 0.0 0 0)
    (Input|RemoveMappingContext (PlayerController|LocalPlayerSubsystems|GetEnhancedInputLocalPlayerSubsystem (Game|GetPlayerController 0)) (Variables|Default|GetPuzzleMapping%20Context) "(bIgnoreAllPressedKeysUntilRelease=True,bForceImmediately=False,bNotifyUserSettings=False)")
    (CallFunction|SetSelectedDiscHighlight false)
    (CallFunction|EmissionAnimation)
    (Utilities|FlowControl|Delay 3.0)
    (UserInterface|Animation|PlayAnimation _wbp_starrotatepuzzle (Variables|/Game/BP/StarPuzzle/WBP_StarRotatePuzzle.WBP_StarRotatePuzzle_C|GetFadeInOut _wbp_starrotatepuzzle) 0.0 1 "Reverse" 1.0 false)
    (Utilities|FlowControl|Delay 1.0)
    (Widget|RemovefromParent _wbp_starrotatepuzzle)
    (Game|Player|SetViewTargetwithBlend (Game|GetPlayerController 0) (Variables|Default|GetCam) 0.0 "VTBlend_Linear" 0.0 false)
    (Utilities|FlowControl|Delay 0.5)
    (bind _opendoor (Timeline|Timeline_0 Play)
      (:Update
        (Transformation|SetRelativeRotation (Variables|Default|GetDoor) (Math|Rotator|MakeRotator (* _opendoor (Variables|Default|GetOpenAngle)) 0.0 0.0) false false)
        (Variables|Default|SetCanBePossessed? false)
        (Variables|Default|SetSolvedPuzzle true))
      (:Finished
        (Utilities|FlowControl|Delay 1.0)
        (CallFunction|ReturntoCharacter)))
    (else
      (Audio|PlaySound2D 0 1.0 1.0 0.0 0 0)
      (Input|RemoveMappingContext (PlayerController|LocalPlayerSubsystems|GetEnhancedInputLocalPlayerSubsystem (Game|GetPlayerController 0)) (Variables|Default|GetPuzzleMapping%20Context) "(bIgnoreAllPressedKeysUntilRelease=True,bForceImmediately=False,bNotifyUserSettings=False)")
      (bind _returnvalue (UserInterface|CreateWidget "/Game/UI/Textbox/WBP_Textbox.WBP_Textbox_C" 0 (Variables|Default|GetRow%20Number) (Variables|Default|GetData%20Table) (Variables|Default|GetEnd%20Of%20Row)))
      (bind _output_get (Variables|Default|SetTextbox _returnvalue))
      (UserInterface|Viewport|AddtoViewport _output_get 0)
      (EventDispatchers|BindEventtoOnEndText _output_get (delegate Custom|EndText)))))

(event EventBeginPlay
  (|CallParentFunction)
  (Variables|Default|SetDiscs (Utilities|Array|MakeArray (Variables|Default|GetBP_RotateRing) (Variables|Default|GetBP_RotateRing1) (Variables|Default|GetBP_RotateRing2)))
  (bind _returnvalue (Rendering|Material|CreateDynamicMaterialInstance (Variables|Default|GetPlane1) 0 "/Game/UI/PuzzlesUI/MI_ZodiacSign.MI_ZodiacSign" "None" :!class /Script/Engine.PrimitiveComponent))
  (Variables|Default|SetMID _returnvalue))

(event EventReturntoCharacter
  (|CallParentFunction))

(fn ConstructionScript)

(fn Interact
  (params (PlayerCharacter :type BP%20First%20Person%20Character%20Object%20Reference))
  (|CallParentFunction PlayerCharacter)
  (if (Variables|Default|GetSolvedPuzzle)
    (CallFunction|SetSelectedDiscHighlight false)
    (return false)
    (else
      (CallFunction|Delay)
      (CallFunction|SetSelectedDiscHighlight true))))

(fn GetSelectedDisc
  (return (Utilities|Array|Get(acopy) (Variables|Default|GetDiscs) (Variables|Default|GetSelectedRingIndex))))

(fn SetSelectedDiscHighlight
  (params (Enable :type Boolean))
  (CallFunction|SetHighlight Enable (CallFunction|GetSelectedDisc)))

(fn ChangeSelectedDisc
  (params (bPickA :type Boolean))
  (CallFunction|SetSelectedDiscHighlight false)
  (Variables|Default|SetSelectedRingIndex (Math|Integer|Clamp(Integer) (+ (Variables|Default|GetSelectedRingIndex) (Math|Integer|SelectInt 1 -1 bPickA)) 0 (Utilities|Array|LastIndex (Variables|Default|GetDiscs))))
  (CallFunction|SetSelectedDiscHighlight true))

(fn EvaluateCombination
  (for (_array_element _array_index) (Variables|Default|GetDiscs)
    (if (Utilities|Enum|NotEqual(Enum) (Default|GetCurrentNumber _array_element) (Utilities|Array|Get(acopy) (Variables|Default|GetCorrectCode) _array_index))
      (return false)))
  (return true))